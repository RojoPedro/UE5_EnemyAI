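; Base enemy character that provides sword combat, patrol route access and movement speed control.
; Attack plays a slash montage and fires OnAttackEnded on completion or interruption.
; Equip and unequip montages use notifies to spawn the sword mesh on the hand socket or destroy it, then update HasWeapon and fire dispatchers on completion.
; SetWalkSpeed maps a gait enum from still to sprinting onto MaxWalkSpeed, and GetPatrolRoute returns the assigned route.
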(event `Attack`
  (`|PlayMontage` (`self.Mesh`) "/Game/Animations/Melee/Montage_Sword_Slash.Montage_Sword_Slash"
    (:`OnCompleted`
      _)
    (:`OnInterrupted`
      _))
  (`self.OnAttackEnded`))

(event `EquipWeapon`
  (bind _notifyname (`|PlayMontage` (`self.Mesh`) "/Game/Animations/Melee/Montage_Unsheath_Sword.Montage_Unsheath_Sword")
    (:`OnCompleted`
      (set `self.HasWeapon` true)
      (`self.OnWeaponEquipped`))
    (:`OnNotifyBegin`
      (switch `name` _notifyname
        (:`HoldSword`
          (bind _returnvalue (`AddComponent|NODE_AddStaticMeshComponent-1` :`bManualAttachment` true))
          (bind _output_get (set `self.Weapon` _returnvalue))
          (`StaticMeshComponent.SetStaticMesh` _output_get "/Game/Assets/Weapons/SM_Sword.SM_Sword")
          (`SceneComponent.K2_AttachToComponent` _returnvalue (`self.Mesh`) "sword_r" "KeepRelative" "KeepRelative" "KeepRelative" true))))))

(event `Unequip Weapon`
  (bind _notifyname (`|PlayMontage` (`self.Mesh`) "/Game/Animations/Melee/Montage_Sheath_Sword.Montage_Sheath_Sword")
    (:`OnCompleted`
      (set `self.HasWeapon` false)
      (`self.OnWeaponUnequipped`))
    (:`OnNotifyBegin`
      (switch `name` _notifyname
        (:`DropSword`
          (`ActorComponent.K2_DestroyComponent` (`self.Weapon`)))))))

(fn `GetPatrolRoute`
  (returns (AssociatedPatrolRoute :type "/Game/AI/Enemy/BP_PatrolRoute Object Reference"))
  (return (`self.PatrolRoute`)))

(fn `SetWalkSpeed`
  (params (NewWalkSpeed :type "/Game/AI/Enemy/ENUM/E_EnemyAI_WalkSpeed Enum" :default "NewEnumerator0"))
  (returns (speed :type "Float (double-precision)"))
  (bind _output_get (set `CharacterMovementComponent.MaxWalkSpeed` (select `/Game/AI/Enemy/ENUM/E_EnemyAI_WalkSpeed` NewWalkSpeed :`NewEnumerator1` 100.0 :`NewEnumerator2` 300.0 :`NewEnumerator3` 500.0) (`self.CharacterMovement`)))
  (return _output_get))

(fn `UserConstructionScript`)