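; Enemy AI controller that runs BT_EnemyAI and turns perception stimuli into blackboard states.
; On each perception update it checks sight, hearing and damage per actor through a shared CanSenseActor helper.
; While Passive or Investigating, seeing the player sets Attacking with a target, and a sound sets Investigating with a point of interest.
; Damage only prints a debug message.
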(event `self.ReceivePossess`
  (params (PossessedPawn :type "Pawn Object Reference"))
  (`KismetSystemLibrary.DelayUntilNextTick`)
  (`self.RunBehaviorTree` "/Game/AI/Enemy/BT_EnemyAI.BT_EnemyAI"))

(event `self.AIPerception.OnPerceptionUpdated`
  (params (UpdatedActors :type "Array of Actor Object Reference (by ref)"))
  ; For each sensed actor
  (for _array_element UpdatedActors
    ; Foreach sense
    (`|ExecutionSequence`
      (:`then_0`
        ; If this sense was triggered
        (bind _result (`self.CanSenseActor` _array_element "NewEnumerator1"))
        (if _result
          ; Right
          (`self.Handle Sensed Sight` _array_element)))
      (:`then_1`
        (bind (_result_2 _stimulusdata) (`self.CanSenseActor` _array_element "NewEnumerator2"))
        (if _result_2
          (`self.HandleSensedSound` (`.StimulusLocation` (break `AIStimulus` _stimulusdata)))))
      (:`then_2`
        (bind _result_3 (`self.CanSenseActor` _array_element "NewEnumerator3"))
        (if _result_3
          (`KismetSystemLibrary.PrintString` "Actor Dealt Damage"))))))

(fn `CanSenseActor`
  (params (Actor :type "Actor Object Reference") (Sense :type "/Game/AI/Enemy/ENUM/E_EnemyAI_Senses Enum" :default "NewEnumerator0"))
  (returns (Result :type Boolean) (StimulusData :type "AIStimulus Structure"))
  ; Get what Sense was triggered by a given actor
  (bind _info (`AIPerceptionComponent.GetActorsPerception` (`self.AIPerception`) Actor))
  ; Check if the stimulus is in our list
  (for _array_element (`.LastSensedStimuli` (break `ActorPerceptionBlueprintInfo` _info))
    (bind _returnvalue (`AIPerceptionSystem.GetSenseClassForStimulus` _array_element))
    (if (== _returnvalue (select `/Game/AI/Enemy/ENUM/E_EnemyAI_Senses` Sense :`NewEnumerator1` "/Script/AIModule.AISense_Sight" :`NewEnumerator2` "/Script/AIModule.AISense_Hearing" :`NewEnumerator3` "/Script/AIModule.AISense_Damage" :!type "Object Class Reference"))
      ; If so, return if sensed or not
      (return (`.bSuccessfullySensed` (break `AIStimulus` _array_element)) _array_element))))

(fn `GetCurrentState`
  (returns (CurrentState :type "/Game/AI/Enemy/ENUM/E_EnemyAI_States Enum"))
  (return (cast `/Game/AI/Enemy/ENUM/E_EnemyAI_States` (`BlackboardComponent.GetValueAsEnum` (`self.Blackboard`) "State"))))

(fn `Handle Sensed Sight`
  (params (SensedActor :type "Actor Object Reference"))
  (switch `/Game/AI/Enemy/ENUM/E_EnemyAI_States` (`self.GetCurrentState`)
    (:`NewEnumerator0`
      _)
    (:`NewEnumerator3`
      _))
  ; If it's the Player
  (if (== SensedActor (`GameplayStatics.GetPlayerCharacter` 0))
    (`self.SetStateAsAttacking` SensedActor)))

(fn `HandleSensedSound`
  (params (SoundLocation :type "Vector Structure"))
  (switch `/Game/AI/Enemy/ENUM/E_EnemyAI_States` (`self.GetCurrentState`)
    (:`NewEnumerator0`
      _)
    (:`NewEnumerator3`
      _))
  (`self.SetStateAsInvestigating` SoundLocation))

(fn `SetStateAsAttacking`
  (params (NewAttackTarget :type "Actor Object Reference"))
  (`BlackboardComponent.SetValueAsEnum` (`self.Blackboard`) "State" (enumliteral `/Game/AI/Enemy/ENUM/E_EnemyAI_States` "NewEnumerator1"))
  (`BlackboardComponent.SetValueAsObject` (`self.Blackboard`) "TargetActor" NewAttackTarget))

(fn `SetStateAsInvestigating`
  (params (InputPin :type "Vector Structure"))
  (`BlackboardComponent.SetValueAsEnum` (`self.Blackboard`) "State" (enumliteral `/Game/AI/Enemy/ENUM/E_EnemyAI_States` "NewEnumerator3"))
  (`BlackboardComponent.SetValueAsVector` (`self.Blackboard`) "PointOfInterest" InputPin))

(fn `SetStateAsPassive`
  (`BlackboardComponent.SetValueAsEnum` (`self.Blackboard`) "State" (enumliteral `/Game/AI/Enemy/ENUM/E_EnemyAI_States` "NewEnumerator0")))

(fn `UserConstructionScript`)